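; AI controller for TrashMonster1 that keeps its possessed monster walking forward and provides logic to turn it around at obstacles.
; It caches the pawn on possession and calls its MoveForward every tick.
; NewFunction runs a forward Visibility line trace, flags InRange for hits closer than a short threshold, and calls TurnChar to rotate the monster 180 degrees.
; Nothing in this controller's own graphs calls NewFunction.
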(event EventTick
  (params (DeltaSeconds :type Float%20%28single-precision%29))
  (bind _as_trash_monster_1 (Variables|Default|GetAs%20Trash%20Monster%201)
    (:then
      (Default|MoveForward _as_trash_monster_1))
    (:else)))

(event EventPossess
  (params (PossessedPawn :type Pawn%20Object%20Reference))
  (bind _astrash_monster_1 (Utilities|Casting|CastToTrashMonster1 PossessedPawn))
  (Variables|Default|SetAs%20Trash%20Monster%201 _astrash_monster_1))

(fn ConstructionScript)

(fn TurnChar
  (bind _as_trash_monster_1 (Variables|Default|GetAs%20Trash%20Monster%201)
    (:then
      (Transformation|SetActorRotation _as_trash_monster_1 (Math|Rotator|CombineRotators (Transformation|GetActorRotation _as_trash_monster_1) "0.000000,180.000000,0.000000")))
    (:else)))

(fn NewFunction
  (params (self2 :type Actor%20Object%20Reference) (self3 :type Actor%20Object%20Reference))
  (bind _returnvalue (Transformation|GetActorLocation self3))
  (bind (_outhit _returnvalue_2) (Collision|LineTraceByChannel _returnvalue (+ _returnvalue (* (Math|Vector|GetForwardVector (Transformation|GetActorRotation self2)) (Variables|Default|GetTraceDistance))) "TraceTypeQuery1" false 0 "None"))
  (if _returnvalue_2
    (Variables|Default|SetDistance (.Distance (Collision|BreakHitResult _outhit)))
    (if (< (.Distance (Collision|BreakHitResult _outhit)) 25.0)
      (Variables|Default|SetInRange true)
      (CallFunction|TurnChar)
      (else
        (Variables|Default|SetInRange false :!label _label)))
    (else
      (goto _label))))