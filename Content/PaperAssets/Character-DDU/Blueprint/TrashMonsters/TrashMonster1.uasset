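; TrashMonster1 is a patrolling monster that walks along its facing direction and turns around at obstacles and edges.
; MoveForward supplies forward movement input, though nothing in this Blueprint calls it.
; Each Tick, a forward visibility trace records hit distance and an InRange flag, flipping the monster on close hits.
; TurnChar rotates it 180 degrees, also triggered by WallDetector overlapping WhitePlayer or any LedgeDetector end overlap.
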(event OnComponentBeginOverlap(WallDetector)
  (params (OverlappedComponent :type Primitive%20Component%20Object%20Reference) (OtherActor :type Actor%20Object%20Reference) (OtherComp :type Primitive%20Component%20Object%20Reference) (OtherBodyIndex :type Integer) (bFromSweep :type Boolean) (SweepResult :type Hit%20Result%20Structure%20%28by%20ref%29))
  (Utilities|Casting|CastToWhitePlayer OtherActor)
  (CallFunction|TurnChar))

(event OnComponentEndOverlap(LedgeDetector)
  (params (OverlappedComponent :type Primitive%20Component%20Object%20Reference) (OtherActor :type Actor%20Object%20Reference) (OtherComp :type Primitive%20Component%20Object%20Reference) (OtherBodyIndex :type Integer))
  (CallFunction|TurnChar))

(event Custom|MoveForward
  (Pawn|Input|AddMovementInput (Transformation|GetActorForwardVector) 1.0 false))

(event EventBeginPlay)

(event Collision|EventActorBeginOverlap
  (params (OtherActor :type Actor%20Object%20Reference)))

(event EventTick
  (params (DeltaSeconds :type Float%20%28single-precision%29))
  (CallFunction|LineTracer))

(fn ConstructionScript)

(fn TurnChar
  (Transformation|SetActorRotation (Math|Rotator|CombineRotators (Transformation|GetActorRotation) "0.000000,180.000000,0.000000")))

(fn LineTracer
  (bind _returnvalue (Transformation|GetActorLocation))
  (bind (_outhit _returnvalue_2) (Collision|LineTraceByChannel _returnvalue (+ _returnvalue (* (Math|Vector|GetForwardVector (Transformation|GetActorRotation)) (Variables|Default|GetTraceDistance))) "TraceTypeQuery1" false 0 "None"))
  (if _returnvalue_2
    (Variables|Default|SetDistance (.Distance (Collision|BreakHitResult _outhit)))
    (if (< (.Distance (Collision|BreakHitResult _outhit)) 25.0)
      (Variables|Default|SetInRange true)
      (CallFunction|TurnChar)
      (else
        (Variables|Default|SetInRange false :!label _label)))
    (else
      (goto _label))))