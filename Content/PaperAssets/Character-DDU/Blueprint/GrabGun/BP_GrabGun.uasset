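; BP_GrabGun is a grab gun pickup that equips itself on the player's WhitePlayer character.
; Its Pickup event detaches any item in the player's Equip slot and re-applies the gun's own root transform.
; It then stores itself in Equip and snaps onto the "GrabGun" socket of the player's Paper2D sprite.
; The graph holds only this equip logic, with no grab or firing behavior.
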(event EventPickup
  (bind _returnvalue (Game|GetPlayerCharacter 0))
  (bind _defaultsceneroot (Variables|Default|GetDefaultSceneRoot))
  (bind _aswhite_player (Utilities|Casting|CastToWhitePlayer _returnvalue))
  (Utilities|IsValid (Variables|/Game/PaperAssets/Character-DDU/Blueprint/Players/WhitePlayer.WhitePlayer_C|GetEquip (.AsWhite%20Player (Utilities|Casting|CastToWhitePlayer (Game|GetPlayerCharacter 0))))
    (:Is%20Valid
      (Transformation|DetachFromActor (Variables|/Game/PaperAssets/Character-DDU/Blueprint/Players/WhitePlayer.WhitePlayer_C|GetEquip (.AsWhite%20Player (Utilities|Casting|CastToWhitePlayer (Game|GetPlayerCharacter 0)))) "KeepRelative" "KeepRelative" "KeepRelative")
      (Transformation|SetActorLocationAndRotation (Transformation|GetWorldLocation _defaultsceneroot) (Transformation|GetWorldRotation _defaultsceneroot)))
    (:Is%20Not%20Valid
      _))
  (Variables|/Game/PaperAssets/Character-DDU/Blueprint/Players/WhitePlayer.WhitePlayer_C|SetEquip _aswhite_player self)
  (Transformation|AttachComponentToComponent (Variables|/Script/Paper2D.PaperCharacter|GetSprite _aswhite_player) "GrabGun" "SnapToTarget" "SnapToTarget" "KeepRelative" true))

(fn ConstructionScript)