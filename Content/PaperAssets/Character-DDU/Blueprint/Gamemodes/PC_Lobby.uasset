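; Lobby player controller that shows the lobby menu and handles leaving a session.
; On BeginPlay, a local controller shows the mouse cursor, switches to UI-only input and opens the menu, which can also be opened through the CreateLobbyMenu event.
; The menu widget is created once, cached and added to the viewport.
; EndClientSession destroys the session and, once that call proceeds, loads the main menu map.
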(event Custom|EndClientSession
  (|DestroySession self
    (:then
      (Game|OpenLevel(byObjectReference) "/Game/Maps/Map_MainMenu.Map_MainMenu"))))

(event Custom|CreateLobbyMenu
  (CallFunction|UIShowLobbyMenu))

(event EventBeginPlay
  (if (Pawn|IsLocalController)
    (Variables|Default|SetbShowMouseCursor true)
    (Input|SetInputModeUIOnly self 0 "DoNotLock" false)
    (CallFunction|UIShowLobbyMenu)))

(fn ConstructionScript)

(fn UIShowLobbyMenu
  (Utilities|IsValid (Variables|Default|GetWB_LobbyMenu)
    (:Is%20Valid
      _)
    (:Is%20Not%20Valid
      (bind _returnvalue (Game|ConstructObjectfromClass self "/Game/UI/WB_Lobby.WB_Lobby_C"))
      (Variables|Default|SetWB_LobbyMenu _returnvalue)))
  (UserInterface|Viewport|AddtoViewport (Variables|Default|GetWB_LobbyMenu) 0)
  (return))