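; Game instance blueprint that handles multiplayer session hosting and server map travel.
; HostSession creates an Advanced Session with a custom server name and slot count, then opens the lobby map as a listen server, printing a message on failure.
; TravelToMap stores the connected player count and runs a Servertravel console command built from the given map name.
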(event Custom|HostSession
  (params (ServerName :type String) (AmountOfSlots :type Integer))
  (|AdvancedSession (Utilities|Array|MakeArray (Class|AdvancedSessionsLibrary|MakeLiteralSessionPropertyString "ServerName" ServerName)) (Game|GetPlayerController 0) AmountOfSlots 0 false true false true true true false false false true false true
    (:OnSuccess
      (Game|OpenLevel(byObjectReference) "/Game/Maps/Map_lobby.Map_lobby" true "listen"))
    (:OnFailure
      (Development|PrintString "Fail"))))

(event Custom|TravelToMap
  (params (NumConnectedPlayers :type Integer) (MapName :type String))
  (Variables|Default|SetNum%20Connected%20Players NumConnectedPlayers)
  (Development|ExecuteConsoleCommand (Utilities|String|Append "Servertravel " MapName) (Game|GetPlayerController 0)))